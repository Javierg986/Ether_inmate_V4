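; BP_HoloPad is a pickup item that projects a configurable hologram mesh above its base, lit by a matching colored light.
; The construction script spawns the mesh at HoloSpawnPoint plus an elevation offset, applying a dynamic hologram material to every slot.
; It auto-scales the hologram from the height bounds of the base and holo meshes, times HoloScale.
; On Pickup, it hides the light and destroys the hologram.
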(event EventBeginPlay
  (|CallParentFunction) ; This node is disabled and will not be called.\nDrag off pins to build functionality.
)

(event Collision|EventActorBeginOverlap
  (params (OtherActor :type Actor%20Object%20Reference))
  (|CallParentFunction OtherActor) ; This node is disabled and will not be called.\nDrag off pins to build functionality.
)

(event EventTick
  (params (DeltaSeconds :type Float%20%28single-precision%29))
  (|CallParentFunction DeltaSeconds) ; This node is disabled and will not be called.\nDrag off pins to build functionality.
)

(event EventPickup
  (params (AttachedTo :type Scene%20Component%20Object%20Reference))
  (|CallParentFunction AttachedTo)
  (Utilities|IsValid (Variables|Default|GetHoloMeshReference)
    (:Is%20Valid
      (Rendering|SetVisibility (Variables|Default|GetHoloLight) false false)
      (Components|DestroyComponent (Variables|Default|GetHoloMeshReference)))))

(fn ConstructionScript
  (bind _holomesh (Variables|Hologram|GetHoloMesh))
  (bind _holospawnpoint (Variables|Default|GetHoloSpawnPoint))
  (bind _holocolor (Variables|Hologram|GetHoloColor))
  (bind _returnvalue (Transformation|GetRelativeTransform _holospawnpoint))
  (bind _returnvalue_2 (Utilities|IsValid _holomesh))
  (bind (_x _y _z) (Math|Vector|BreakVector (.location _returnvalue)))
  (|CallParentFunction)
  ;[1 1 1] Check if there is a valid Holo Mesh
  (Rendering|SetVisibility (Variables|Default|GetHoloLight) _returnvalue_2 false)
  (if _returnvalue_2
    ;[1 1 1] Set Holo Mesh
    (bind _returnvalue_3 (AddComponent|AddStaticMeshComponent false (Math|Transform|MakeTransform (Math|Vector|MakeVector _x _y (+ _z (Variables|Hologram|GetHoloMeshElevationOffset))) (Variables|Hologram|GetHoloMeshRotation) (.scale _returnvalue))))
    (bind _output_get (Variables|Default|SetHoloMeshReference _returnvalue_3))
    (Components|StaticMesh|SetStaticMesh _output_get (Variables|Hologram|GetHoloMesh))
    ;[1 1 1] Create & Add Holo Material
    (bind _returnvalue_4 (Rendering|Material|CreateDynamicMaterialInstance _returnvalue_3 0 "/Game/ScifiOutpost/Materials/Effects/M_HoloItem.M_HoloItem" "None" :!class /Script/Engine.PrimitiveComponent))
    (Variables|Hologram|SetHoloMatInst _returnvalue_4)
    (for _index (range 0 (- (Rendering|Material|GetNumMaterials _returnvalue_3) 1))
      (Rendering|Material|SetMaterial _returnvalue_3 _index (Variables|Hologram|GetHoloMatInst))
      ;[1 1 1] Set Material & Light Parameters
      (Rendering|Material|SetVectorParameterValue (Variables|Hologram|GetHoloMatInst) "HologramColor" _holocolor :!class /Script/Engine.MaterialInstanceDynamic)
      (Rendering|Components|Light|SetLightColor (Variables|Default|GetHoloLight) _holocolor true)
      ;[1 1 1] Scale Mesh to Match with the Base Mesh
      (Transformation|SetRelativeScale3D _returnvalue_3 (* "1.000000,1.000000,1.000000" (* (/ (.Z (Math|Vector|BreakVector (.Max (Components|StaticMesh|GetLocalBounds (Variables|Default|GetItemMesh))))) (.Z (Math|Vector|BreakVector (.Max (Components|StaticMesh|GetLocalBounds _returnvalue_3))))) (Variables|Hologram|GetHoloScale)))))))