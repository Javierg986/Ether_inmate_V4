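; Parent Blueprint for a fog sheet, a mesh-based fog effect placed in the environment and built in the construction script.
; SetFogValues creates a dynamic material instance from FogMaterial and pushes the exposed texture, color, wind, emissive, opacity and micro/macro noise settings into it.
; GenerateFogSheet then adds a scaled static mesh under FogSheets with that material, using EditorPlane when no FogMesh is set.
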(fn ConstructionScript
  (CallFunction|SetFogValues)
  (CallFunction|GenerateFogSheet))

(fn GenerateFogSheet
  (bind _returnvalue (AddComponent|AddStaticMeshComponent false (Math|Transform|MakeTransform "0, 0, 0" "0, 0, 0" (Variables|FogMesh|GetFogSheetScale)))) ; Create fogsheet mesh
  (Rendering|Material|SetMaterial _returnvalue 0 (Variables|Material|GetFogSheetMatIns))
  (Components|StaticMesh|SetStaticMesh _returnvalue (select (Utilities|IsValid (Variables|FogMesh|GetFogMesh)) (Variables|FogMesh|GetFogMesh) "/Engine/EditorMeshes/EditorPlane.EditorPlane"))
  (Transformation|AttachComponentToComponent _returnvalue (Variables|Default|GetFogSheets) "None" "KeepRelative" "KeepRelative" "KeepRelative" true))

(fn SetFogValues
  (bind _returnvalue (Rendering|Material|CreateDynamicMaterialInstance (Variables|Material|GetFogMaterial) "None" "None" :!class /Script/Engine.KismetMaterialLibrary))
  (bind _output_get (Variables|Material|SetFogSheetMatIns _returnvalue))
  ;[1 1 1] Textures
  (Rendering|Material|SetTextureParameterValue _output_get "MacroFogNormal" (Variables|FogControl|Textures|GetMacroFogNormal))
  (Rendering|Material|SetTextureParameterValue _output_get "FogMainNoise" (Variables|FogControl|Textures|GetFogMainNoise))
  (Rendering|Material|SetTextureParameterValue _output_get "FogShapeMask" (Variables|FogControl|Textures|GetFogShapeMask))
  (Rendering|Material|SetScalarParameterValue _output_get "MacroFogNormalAmount" (Variables|FogControl|Textures|GetNormalntensity) :!class /Script/Engine.MaterialInstanceDynamic)
  (Rendering|Material|SetVectorParameterValue _output_get "FogColor" (Variables|FogControl|Color|GetFogColor) :!class /Script/Engine.MaterialInstanceDynamic)
  ;[1 1 1] Wind
  (Rendering|Material|SetVectorParameterValue _output_get "WIndDirection" (Variables|FogControl|Wind|GetWindDirection) :!class /Script/Engine.MaterialInstanceDynamic)
  (Rendering|Material|SetScalarParameterValue _output_get "WindSpeed" (Variables|FogControl|Wind|GetWindSpeed) :!class /Script/Engine.MaterialInstanceDynamic)
  ;[1 1 1] Emissive
  (Rendering|Material|SetScalarParameterValue _output_get "FakeEmissiveMultiplier" (Variables|FogControl|Emissive|GetEmissiveMultiplier) :!class /Script/Engine.MaterialInstanceDynamic)
  ;[1 1 1] Opacity
  (Rendering|Material|SetScalarParameterValue _output_get "Opacity" (Variables|FogControl|Opacity|GetOpacity) :!class /Script/Engine.MaterialInstanceDynamic)
  (Rendering|Material|SetScalarParameterValue _output_get "SphereMaskHardness" (Variables|FogControl|Shape|GetSphereMaskHardness) :!class /Script/Engine.MaterialInstanceDynamic)
  (Rendering|Material|SetScalarParameterValue _output_get "SphereMaskRadius" (Variables|FogControl|Shape|GetSphereMaskRadius) :!class /Script/Engine.MaterialInstanceDynamic)
  (Rendering|Material|SetScalarParameterValue _output_get "ShapeMaskAlpha" (Variables|FogControl|Shape|GetShapeMaskAlpha) :!class /Script/Engine.MaterialInstanceDynamic)
  (Rendering|Material|SetScalarParameterValue _output_get "OpacityFactor" (Variables|FogControl|Fading|GetOpacityFactor) :!class /Script/Engine.MaterialInstanceDynamic)
  (Rendering|Material|SetScalarParameterValue _output_get "DeepnessFade" (Variables|FogControl|Fading|GetDeepnessFade) :!class /Script/Engine.MaterialInstanceDynamic)
  ;[1 1 1] Micro Fog
  (Rendering|Material|SetScalarParameterValue _output_get "MicroFogScale" (Variables|FogControl|MicroFog|GetMicroFogScale) :!class /Script/Engine.MaterialInstanceDynamic)
  (Rendering|Material|SetScalarParameterValue _output_get "MicroFogSpeedOffset" (Variables|FogControl|MicroFog|GetMicroFogSpeedOffset) :!class /Script/Engine.MaterialInstanceDynamic)
  (Rendering|Material|SetScalarParameterValue _output_get "MicroFogContrast" (Variables|FogControl|MicroFog|GetMicroFogContrast) :!class /Script/Engine.MaterialInstanceDynamic)
  ;[1 1 1] Macro Fog
  (Rendering|Material|SetScalarParameterValue _output_get "MacroFogScale" (Variables|FogControl|MacroFog|GetMacroFogScale) :!class /Script/Engine.MaterialInstanceDynamic)
  (Rendering|Material|SetScalarParameterValue _output_get "MacroFogSpeedOffset" (Variables|FogControl|MacroFog|GetMacroFogSpeedOffset) :!class /Script/Engine.MaterialInstanceDynamic)
  (Rendering|Material|SetScalarParameterValue _output_get "MacroFogContrast" (Variables|FogControl|MacroFog|GetMacroFogContrast) :!class /Script/Engine.MaterialInstanceDynamic)
  (Rendering|Material|SetScalarParameterValue _output_get "MacroFogAlpha" (Variables|FogControl|MacroFog|GetMacroFogAlpha) :!class /Script/Engine.MaterialInstanceDynamic)
  (Rendering|Material|SetScalarParameterValue _output_get "FogMaskMultiplier" (Variables|FogControl|Opacity|GetFogMaskMultiplier) :!class /Script/Engine.MaterialInstanceDynamic))