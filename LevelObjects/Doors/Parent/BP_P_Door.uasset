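; Parent door Blueprint for level doors that sets up each door's look at construction time.
; The construction script runs the parent script, then InitDoors and InitDoorVisuals, which applies the Visuals settings to a valid Door mesh.
; DetailMesh receives default custom primitive data for a power-off flag and a red locked or blue unlocked color, based on the first DoorDataset entry.
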(event Collision|EventActorBeginOverlap
  (params (OtherActor :type Actor%20Object%20Reference)))

(event EventTick
  (params (DeltaSeconds :type Float%20%28single-precision%29)))

(fn ConstructionScript
  (|CallParentFunction)
  (CallFunction|InitDoors)
  (CallFunction|InitDoorVisuals))

(fn InitDoorVisuals
  (bind _door (Variables|Default|GetDoor))
  (bind _doordataset (Variables|Default|GetDoorDataset))
  (bind _detailmesh (Variables|Default|GetDetailMesh))
  (bind _output (Utilities|Array|Get(acopy) _doordataset))
  (bind _returnvalue (select (.doorlocked _output) "(R=1.000000,G=0.000000,B=0.000000,A=1.000000)" "(R=0.000000,G=0.392157,B=1.000000,A=1.000000)"))
  (bind (_r _g _b _a) (Math|Color|BreakColor _returnvalue))
  (Utilities|IsValid _door
    (:Is%20Valid
      (Utilities|SetPrimitiveVisuals (Variables|Control|Appearance|GetVisuals) _door
        (:Out
          _)))
    (:Is%20Not%20Valid
      _))
  (Rendering|Material|SetDefaultCustomPrimitiveDataFloat _detailmesh 20 (select (Variables|Default|GetIsPowerOn) 0.0 1.0))
  (Rendering|Material|SetDefaultCustomPrimitiveDataVector4 _detailmesh 16 (Math|Vector4|MakeVector4 _r _g _b _a)))