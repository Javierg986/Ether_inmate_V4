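; Parent Blueprint for light level objects that switch on and off and can be given a color and visual style.
; ToggleLight writes on/off state and color to the DetailMesh's custom primitive data for its material, and sets color and visibility on light components under Lights.
; Construction applies it from IsPowerOn and restyles the meshes through SetPrimitiveVisuals.
; Activate reapplies it from IsActive.
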(event EventBeginPlay
  (|CallParentFunction) ; This node is disabled and will not be called.\nDrag off pins to build functionality.
)

(event Collision|EventActorBeginOverlap
  (params (OtherActor :type Actor%20Object%20Reference))
  (|CallParentFunction OtherActor) ; This node is disabled and will not be called.\nDrag off pins to build functionality.
)

(event EventTick
  (params (DeltaSeconds :type Float%20%28single-precision%29))
  (|CallParentFunction DeltaSeconds) ; This node is disabled and will not be called.\nDrag off pins to build functionality.
)

(event EventActivate
  (|CallParentFunction)
  (CallFunction|ToggleLight (Variables|Default|GetIsActive) (Variables|Default|GetLightColor)))

(fn ConstructionScript
  (|CallParentFunction)
  (CallFunction|ToggleLight (Variables|Default|GetIsPowerOn) (Variables|Default|GetLightColor))
  (CallFunction|EditApperance))

(fn ToggleLight
  (params (LightVisibility :type Boolean) (LightColor :type Linear%20Color%20Structure))
  (bind _detailmesh (Variables|Default|GetDetailMesh))
  (bind (_r _g _b _a) (Math|Color|BreakColor (Variables|Default|GetLightColor)))
  ;[1 1 1] Light Material Control
  (Rendering|Material|SetCustomPrimitiveDataFloat _detailmesh 20 (select LightVisibility 0.0 1.0))
  (Rendering|Material|SetCustomPrimitiveDataVector4 _detailmesh 16 (Math|Vector4|MakeVector4 _r _g _b _a))
  ;[1 1 1] Handle Light Components
  (for _array_element (Components|GetChildrenComponents (Variables|Default|GetLights) false)
    (bind _aslight_component (Utilities|Casting|CastToLightComponent _array_element))
    (Rendering|Components|Light|SetLightColor _aslight_component LightColor true)
    (Rendering|SetVisibility _aslight_component LightVisibility false)))

(fn EditApperance
  (for _array_element (Components|GetChildrenComponents (Variables|Default|GetMeshes) true)
    (bind _asstatic_mesh_component (Utilities|Casting|CastToStaticMeshComponent _array_element))
    (Utilities|SetPrimitiveVisuals (Variables|Control|Appearance|GetVisuals) _asstatic_mesh_component))
  (Utilities|SetPrimitiveVisuals (Variables|Control|Appearance|GetVisuals) (Variables|Default|GetBaseMesh)))