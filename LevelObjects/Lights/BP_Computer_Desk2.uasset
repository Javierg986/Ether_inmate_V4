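; Desk computer level object whose screen and light reflect power and active state, built on a parent that provides activation and light toggling.
; The construction script shows the UI and light when powered, using LightColor when active or a fixed red-orange when inactive.
; State and color reach the UI material through custom primitive data.
; On Activate, it runs parent logic, then shows the UI only if both active and powered.
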(event EventBeginPlay
  (|CallParentFunction) ; This node is disabled and will not be called.\nDrag off pins to build functionality.
)

(event Collision|EventActorBeginOverlap
  (params (OtherActor :type Actor%20Object%20Reference))
  (|CallParentFunction OtherActor) ; This node is disabled and will not be called.\nDrag off pins to build functionality.
)

(event EventTick
  (params (DeltaSeconds :type Float%20%28single-precision%29))
  (|CallParentFunction DeltaSeconds) ; This node is disabled and will not be called.\nDrag off pins to build functionality.
)

(event EventActivate
  (|CallParentFunction)
  (Rendering|SetVisibility (Variables|Default|GetUI) (and (Variables|Default|GetIsActive) (Variables|Default|GetIsPowerOn)) false))

(fn ConstructionScript
  (bind _ui (Variables|Default|GetUI))
  (bind _isactive (Variables|Default|GetIsActive))
  (bind _lightcolor (Variables|Default|GetLightColor))
  (bind _returnvalue (select _isactive _lightcolor "(R=1.000000,G=0.051108,B=0.000000,A=1.000000)"))
  (bind (_r _g _b _a) (Math|Color|BreakColor _returnvalue))
  (|CallParentFunction)
  (Rendering|SetVisibility _ui (Variables|Default|GetIsPowerOn) false)
  (Rendering|Material|SetDefaultCustomPrimitiveDataFloat _ui 0 (select _isactive 0.0 1.0))
  (Rendering|Material|SetDefaultCustomPrimitiveDataVector4 _ui 1 (Math|Vector4|MakeVector4 _r _g _b _a))
  (CallFunction|ToggleLight (Variables|Default|GetIsPowerOn) _returnvalue))