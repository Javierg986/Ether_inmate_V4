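; Parent Blueprint for furniture level objects, configured entirely in the construction script.
; It toggles lights from the power state, initializes doors, optionally spawns actors and meshes from prefixed sockets on the base mesh, and initializes random rotation.
; EditAppearance then applies the shared Visuals settings to the base mesh and the static meshes under the Meshes and Doors components.
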(event EventBeginPlay)

(event EventTick
  (params (DeltaSeconds :type Float%20%28single-precision%29))
  (|CallParentFunction DeltaSeconds) ; This node is disabled and will not be called.\nDrag off pins to build functionality.
)

(fn ConstructionScript
  (bind _base (Variables|Default|GetBase))
  (|CallParentFunction)
  (CallFunction|ToggleLights (Variables|Default|GetIsPowerOn) (Variables|Default|GetLights))
  (CallFunction|InitDoors)
  (if (Variables|Default|GetSpawnSocketActors)
    (CallFunction|SpawnActorsfromSockets "Actor" (Variables|Default|GetSocketActorsRotations) (Variables|Default|GetSocketActors) (Variables|/Script/Engine.StaticMeshComponent|GetStaticMesh _base) _base))
  (if (Variables|Default|GetSpawnSocketMeshes)
    (CallFunction|SpawnMeshesfromSockets (Variables|Default|GetSocketHISMs) (Variables|Default|GetSocketMeshes) _base "Mesh"))
  (CallFunction|InitRandomRotation)
  (CallFunction|EditAppearance))

(fn EditAppearance
  (for _array_element (Components|GetChildrenComponents (Variables|Default|GetMeshes) true)
    (bind _asstatic_mesh_component (Utilities|Casting|CastToStaticMeshComponent _array_element))
    (Utilities|SetPrimitiveVisuals (Variables|Control|Appearance|GetVisuals) _asstatic_mesh_component))
  (for _array_element_2 (Components|GetChildrenComponents (Variables|Default|GetDoors) false)
    (bind _asstatic_mesh_component_2 (Utilities|Casting|CastToStaticMeshComponent _array_element_2))
    (Utilities|SetPrimitiveVisuals (Variables|Control|Appearance|GetVisuals) _asstatic_mesh_component_2))
  (Utilities|SetPrimitiveVisuals (Variables|Control|Appearance|GetVisuals) (Variables|Default|GetBase)))