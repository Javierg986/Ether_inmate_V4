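; BP_Pump is a level machine whose piston animates up and down the Z axis in a repeating pump cycle.
; If active and powered at BeginPlay, a looping timer restarts the piston timeline, which drives the piston's relative height.
; A seeded random start-delay variance on the timer staggers pump timing.
; The construction script runs the parent's setup, then calls ToggleEmissive on the base detail.
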(event Custom|Start%20Pumping
  (bind _pistonzmovement (Timeline|PistonMovement PlayFromStart)
    (:Update
      (Transformation|SetRelativeLocation (Variables|Default|GetPiston) (Math|Vector|MakeVector 0.0 0.0 (Math|Float|Lerp 1.3e+03 1.6e+03 _pistonzmovement)) false false))))

(event EventBeginPlay
  (if (and (Variables|Default|GetIsActive) (Variables|Default|GetIsPowerOn))
    (Utilities|Time|SetTimerbyEvent (delegate Custom|Start%20Pumping) 5.0 true false 0.0 (Math|Random|RandomFloatinRangefromStream (Variables|Default|GetRandomSeedStruct) 0.0 2.0))))

(event Collision|EventActorBeginOverlap
  (params (OtherActor :type Actor%20Object%20Reference)))

(event EventTick
  (params (DeltaSeconds :type Float%20%28single-precision%29)))

(fn ConstructionScript
  (|CallParentFunction)
  (CallFunction|ToggleEmissive (Variables|Default|GetBase_Detail)))