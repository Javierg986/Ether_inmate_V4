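; Solar panel machine that turns to track the level's sun while it is powered and active.
; At BeginPlay it takes the first Directional Light found and starts a looping timer that calls LookAt.
; LookAt converts the light's rotation into a local direction, then interpolates Arm yaw and clamped Panel pitch toward it, both starting from the Panel's rotation.
; The construction script calls ToggleEmissive on BaseDetail.
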(event EventBeginPlay
  (CallFunction|UpdateSun)
  (Utilities|Time|SetTimerbyFunctionName 0 "LookAt" (Variables|Default|GetUpdateDelay) true))

(event Collision|EventActorBeginOverlap
  (params (OtherActor :type Actor%20Object%20Reference)))

(event EventTick
  (params (DeltaSeconds :type Float%20%28single-precision%29)))

(fn ConstructionScript
  (|CallParentFunction)
  (CallFunction|ToggleEmissive (Variables|Default|GetBase_Detail)))

(fn Lookat
  (bind _lookingspeed (Variables|LookAt|GetLookingSpeed))
  ;[1 1 1] Rotate to Aim
  (if (Math|Boolean|ANDBoolean (Utilities|IsValid (Variables|LookAt|GetLookAtActor)) (Variables|Default|GetIsPowerOn) (Variables|Default|GetIsActive))
    (bind _output_get (Variables|LookAt|SetLookingAtLocation (Math|Transform|InverseTransformDirection (Transformation|GetActorTransform) (Math|Vector|RotateVector "-10000.000000,-0.000000,0.000000" (Transformation|GetActorRotation (Variables|LookAt|GetLookAtActor))))))
    (Transformation|SetRelativeRotation (Variables|Default|GetArm) (Math|Interpolation|RInterpTo (Variables|/Script/Engine.SceneComponent|GetRelativeRotation (Variables|Default|GetPanel)) (Math|Rotator|MakeRotator 0.0 0.0 (.Yaw (Math|Rotator|BreakRotator (Math|Rotator|MakeRotfromX _output_get)))) (Utilities|Time|GetWorldDeltaSeconds) _lookingspeed) false false)
    (Transformation|SetRelativeRotation (Variables|Default|GetPanel) (Math|Rotator|MakeRotator (.Roll (Math|Rotator|BreakRotator (Math|Interpolation|RInterpTo (Variables|/Script/Engine.SceneComponent|GetRelativeRotation (Variables|Default|GetPanel)) (Math|Rotator|MakeRotator 0.0 (.Pitch (Math|Rotator|BreakRotator (Math|Rotator|MakeRotfromX _output_get))) 0.0) (Utilities|Time|GetWorldDeltaSeconds) _lookingspeed))) (Math|Float|ClampAngle (.Pitch (Math|Rotator|BreakRotator (Math|Interpolation|RInterpTo (Variables|/Script/Engine.SceneComponent|GetRelativeRotation (Variables|Default|GetPanel)) (Math|Rotator|MakeRotator 0.0 (.Pitch (Math|Rotator|BreakRotator (Math|Rotator|MakeRotfromX _output_get))) 0.0) (Utilities|Time|GetWorldDeltaSeconds) _lookingspeed))) (Variables|LookAt|GetLookAtMinAngle) (Variables|LookAt|GetLookAtMaxAngle)) (.Yaw (Math|Rotator|BreakRotator (Math|Interpolation|RInterpTo (Variables|/Script/Engine.SceneComponent|GetRelativeRotation (Variables|Default|GetPanel)) (Math|Rotator|MakeRotator 0.0 (.Pitch (Math|Rotator|BreakRotator (Math|Rotator|MakeRotfromX _output_get))) 0.0) (Utilities|Time|GetWorldDeltaSeconds) _lookingspeed)))) false false)))

(fn UpdateSun
  ;[1 1 1] Get Reference to Directional Light (Sun)
  (bind _outactors (Actor|GetAllActorsOfClass "/Script/Engine.DirectionalLight"))
  (if (Utilities|IsValid (Utilities|Array|Get(acopy) _outactors))
    (Variables|LookAt|SetLookAtActor (Utilities|Array|Get(acopy) _outactors))
    (else
      (Variables|LookAt|SetLookAtActor 0))))